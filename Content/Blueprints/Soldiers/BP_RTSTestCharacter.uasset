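; RTS test soldier that takes move orders and shoots arrows at a placeholder dragon.
; Move orders pass through ServerMoveCharacter to the RTS AI controller as a message.
; Tick searches for the first dragon dummy and, within range, spawns an aimed arrow each frame while re-setting a looping timer.
; That timer's SpawnArrow event feeds back into the same spawn through a delayed loop, with debug prints throughout.
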(event `/Game/Blueprints/Interfaces/BPI_RTSMovable.Move Character To`
  (params (Location :type "Vector Structure"))
  (`self.ServerMoveCharacter` Location))

(event `self.ReceiveBeginPlay`)

(event `ServerMoveCharacter`
  (params (location :type "Vector Structure"))
  ;[1 1 1] Move
  (bind _asrtsaicontroller (cast `/Game/Blueprints/RTS/RTSAIController` (`self.GetController`)))
  (message `/Game/Blueprints/Interfaces/BPI_RTSMovable.Move Character To` _asrtsaicontroller location))

(event `self.ReceiveActorBeginOverlap`
  (params (OtherActor :type "Actor Object Reference")))

(event `self.ReceiveTick`
  (params (DeltaSeconds :type "Float (single-precision)"))
  (bind _returnvalue (+ (* (`KismetMathLibrary.GetForwardVector` (`self.K2_GetActorRotation`)) 30.0) (`self.K2_GetActorLocation`)))
  (bind _outactors (`GameplayStatics.GetAllActorsOfClass` "/Game/Blueprints/Soldiers/BP_TEMPDragonDUMMY.BP_TEMPDragonDUMMY_C"))
  (if (> (`KismetArrayLibrary.Array_Length` _outactors) 0)
    (bind _item (`KismetArrayLibrary.Array_Get` _outactors))
    (`/Engine/EditorBlueprintResources/StandardMacros.IsValid` _item
      (:`Is Valid`
        (bind _returnvalue_2 (- (`SceneComponent.K2_GetComponentLocation` (`Character.Mesh` _item)) _returnvalue))
        (bind _returnvalue_3 (`KismetMathLibrary.VSize` _returnvalue_2))
        (`KismetSystemLibrary.PrintString` (`KismetStringLibrary.Conv_DoubleToString` _returnvalue_3) true true (struct :`G` 0.66 :`B` 1.0 :`A` 1.0) 0.0)
        (if (< _returnvalue_3 200.0)
          (`KismetSystemLibrary.K2_SetTimerDelegate` (delegate `SpawnArrow`) 2.0 true)
          (`|SpawnActorFromClass` "/Game/Blueprints/Soldiers/Arrow.Arrow_C" (`KismetMathLibrary.MakeTransform` _returnvalue (`KismetMathLibrary.MakeRotationFromAxes` _returnvalue_2 (0.0 0.0 0.0) (0.0 0.0 1.0))) "AlwaysSpawn" "OverrideRootScale" :!label _label)
          (`KismetSystemLibrary.PrintString` "arrow spawned"))))))

(event `SpawnArrow`
  (`/Engine/EditorBlueprintResources/StandardMacros.IsValid` (`KismetArrayLibrary.Array_Get` (stale `self.ReceiveTick` _outactors))
    (:`Is Valid`
      (for _ (range 3)
        (`KismetSystemLibrary.Delay` 2.0)
        (goto _label)))))

(fn `UserConstructionScript`)